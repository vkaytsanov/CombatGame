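; Player character Blueprint that creates the HUD on begin play and runs a four-hit light attack montage combo.
; An attack counter selects the next montage when an attack starts, wrapping after the fourth hit.
; A combo animation notify chains into the next montage if CombatPlayerController's ConditionalAdvanceAttack allows it.
; The combo-end notify resets the counter and tells the controller the attack has ended.
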(event `self.ReceiveBeginPlay`
  (bind _returnvalue (`|CreateWidget` "/Game/BlueprintsUI/WB_PlayerHUD.WB_PlayerHUD_C"))
  (`UserWidget.AddToViewport` _returnvalue 0))

(event `self.OnAttackStart_BP`
  ;[1 1 1] Combo System Setup.
  (switch `int` (`self.AttackCount`) :!label _label
    (:`0`
      (set `self.AttackCount` 1)
      (`self.PlayAnimMontage` "/Game/Characters/Kachujin/Animations/LigthAttack/LightAttk1_Montage.LightAttk1_Montage"))
    (:`1`
      (set `self.AttackCount` 2)
      (`self.PlayAnimMontage` "/Game/Characters/Kachujin/Animations/LigthAttack/LightAttk2_Montage.LightAttk2_Montage"))
    (:`2`
      (set `self.AttackCount` 3)
      (`self.PlayAnimMontage` "/Game/Characters/Kachujin/Animations/LigthAttack/LightAttk3_Montage.LightAttk3_Montage"))
    (:`3`
      (set `self.AttackCount` 0)
      (`self.PlayAnimMontage` "/Game/Characters/Kachujin/Animations/LigthAttack/LightAttk4_Montage.LightAttk4_Montage"))))

(event `Notify_Combo_FromAnimation`
  ;[1 1 1] Combo System Setup.
  (bind _returnvalue (`CombatPlayerController.ConditionalAdvanceAttack` (cast `CombatPlayerController` (`GameplayStatics.GetPlayerController` 0) :!pure true)))
  (if _returnvalue
    (goto _label)))

(event `Notify_Combo_End_FromAnimation`
  ;[1 1 1] Combo System Setup.
  (set `self.AttackCount` 0)
  (`CombatPlayerController.OnAttackEnd_BP` (cast `CombatPlayerController` (`GameplayStatics.GetPlayerController` 0) :!pure true)))

(fn `UserConstructionScript`)