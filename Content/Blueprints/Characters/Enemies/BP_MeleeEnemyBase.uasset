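; Base Blueprint for melee enemies that handles visual feedback when the enemy takes damage.
; The OnDamageTakenBP event spawns a damage text widget component showing the amount, then refreshes and reveals the enemy's health bar.
; UpdateHealthbar casts the HealthBarWidget's user widget to WB_EnemyHP, sets its progress from GetHealthBarFillPercent and returns it so the event can make it visible.
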(event `self.OnDamageTaken_BP`
  (params (DamageTaken :type Integer))
  (bind _returnvalue (`AddComponent|NODE_AddWC_DamageText-1`))
  (`/Game/BlueprintsUI/WC_DamageText.SetDamageText` _returnvalue (`KismetMathLibrary.Conv_IntToDouble` DamageTaken))
  (bind _wb_enemyhp (`self.Update Healthbar`))
  (`Widget.SetVisibility` _wb_enemyhp "Visible"))

(fn `Update Healthbar`
  (returns (WB_EnemyHP :type "/Game/BlueprintsUI/WB_EnemyHP Object Reference"))
  (bind _aswb_enemy_hp (cast `/Game/BlueprintsUI/WB_EnemyHP` (`WidgetComponent.GetUserWidgetObject` (`self.HealthBar Widget`))))
  (bind _returnvalue (`/Game/BlueprintsUI/BPL_Characters.Get Health Bar Fill Percent` (`CharacterMovementComponent.GetCharacterOwner` (`self.CharacterMovement`))))
  (`/Game/BlueprintsUI/WB_EnemyHP.SetProgress` _aswb_enemy_hp _returnvalue)
  (return _aswb_enemy_hp))

(fn `UserConstructionScript`)